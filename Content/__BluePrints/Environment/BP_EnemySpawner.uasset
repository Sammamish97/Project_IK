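; BP_EnemySpawner is an environment actor that spawns a batch of enemies when its ActivateSpawner event is called.
; It loops SpawnAmount times, picking random navigable points within the SpawnArea sphere and spawning TargetClass there with InitialRotation.
; Each spawn adjusts for collisions but always spawns, then receives its default AI controller.
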(event Collision|EventActorBeginOverlap
  (params (OtherActor :type Actor%20Object%20Reference)))

(event EventTick
  (params (DeltaSeconds :type Float%20%28single-precision%29)))

(event EventActivateSpawner
  (bind _spawnarea (Variables|Default|GetSpawnArea))
  (for _index (range 0 (- (Variables|Default|Getspawn_amount_) 1))
    (bind _randomlocation (Class|NavigationSystemV1|GetRandomLocationinNavigableRadius (Transformation|GetWorldLocation _spawnarea) (Variables|/Script/Engine.SphereComponent|GetSphereRadius _spawnarea) 0 0))
    (bind _returnvalue (Game|SpawnActorfromClass (Variables|Default|Gettarget_class_) (Math|Transform|MakeTransform _randomlocation (Variables|Default|Getinitial_rotation_) "1.000000,1.000000,1.000000") "AdjustIfPossibleButAlwaysSpawn" "MultiplyWithRoot" 0 0))
    (Pawn|SpawnDefaultController _returnvalue)))

(fn ConstructionScript)