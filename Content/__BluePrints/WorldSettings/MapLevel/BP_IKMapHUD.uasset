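; BP_IKMapHUD is the map level HUD Blueprint that manages showing and hiding the inventory screen.
; On BeginPlay it creates one BP_InventoryWidget, initializes it with the InventoryManager from IKGameInstance and loads its data.
; PopUpInventory reloads from the manager and adds the widget to the viewport.
; RemoveInventory detaches the widget, then applies its state back to the manager.
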(event Custom|PopUpInventory
  (bind _inventorywidget (Variables|Default|GetInventoryWidget))
  (Class|InventoryWidget|LoadInventoryManager _inventorywidget)
  (UserInterface|Viewport|AddtoViewport _inventorywidget 0))

(event Custom|RemoveInventory
  (bind _inventorywidget (Variables|Default|GetInventoryWidget))
  (Widget|RemovefromParent _inventorywidget)
  (Class|InventoryWidget|ApplyInventoryManager _inventorywidget))

(event EventBeginPlay
  (bind _returnvalue (UserInterface|CreateWidget "/Game/__BluePrints/UI/Inventory/Upgraded/BP_InventoryWidget.BP_InventoryWidget_C"))
  (bind _output_get (Variables|Default|SetInventoryWidget _returnvalue))
  (Class|InventoryWidget|InitInventoryWidget _output_get (Class|IKGameInstance|GetInventoryManager (.AsIKGame%20Instance (Utilities|Casting|CastToIKGameInstance (Game|GetGameInstance)))))
  (Class|InventoryWidget|LoadInventoryManager _output_get))

(event Collision|EventActorBeginOverlap
  (params (OtherActor :type Actor%20Object%20Reference)))

(event EventTick
  (params (DeltaSeconds :type Float%20%28single-precision%29)))

(fn ConstructionScript)