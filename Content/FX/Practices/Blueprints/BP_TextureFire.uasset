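; BP_TextureFire is an FX practice actor that pairs a texture-driven Niagara fire with a plane displaying the same texture.
; Its Construction Script feeds the exposed texture, fire color and density into the Niagara component's user parameters.
; It also creates a dynamic instance of the logo material on the plane, setting its texture and tint from the same variables.
; All event graph nodes are unused.
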(event EventBeginPlay)

(event Collision|EventActorBeginOverlap
  (params (OtherActor :type Actor%20Object%20Reference)))

(event EventTick
  (params (DeltaSeconds :type Float%20%28single-precision%29)))

(fn ConstructionScript
  (bind _niagarafire (Variables|Default|GetNiagaraFire))
  (bind _texture (Variables|PacktAttributes|GetTexture))
  (bind _firecolor (Variables|PacktAttributes|GetFireColor))
  (Niagara|SetNiagaraVariable(Float) _niagarafire "User.FireDensity" (Variables|PacktAttributes|GetFireDensity))
  (Class|NiagaraComponent|SetVariableTexture _niagarafire "User.Texture" _texture)
  (bind _returnvalue (Rendering|Material|CreateDynamicMaterialInstance (Variables|Default|GetPlane) 0 "/Game/FX/Practices/Material/M_packtlogo.M_packtlogo" "None" :!class /Script/Engine.PrimitiveComponent))
  (Rendering|Material|SetTextureParameterValue _returnvalue "TextureUsed" _texture)
  (Rendering|Material|SetVectorParameterValue _returnvalue "LogoColor" _firecolor :!class /Script/Engine.MaterialInstanceDynamic)
  (Niagara|SetNiagaraVariable(LinearColor) _niagarafire "User.FireColor" _firecolor))