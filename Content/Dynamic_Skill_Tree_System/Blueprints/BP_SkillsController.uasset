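; Skills controller actor that owns the skill tree menu widget and handles opening and closing it during play.
; On BeginPlay it creates WBP_SkillsMenu and adds it to the viewport after a deliberate zero-second delay.
; Opening or closing the menu also switches mouse cursor, input mode and game pause.
; Open state and skill detail updates pass through messages to the menu and its details widget.
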(event EventBeginPlay
  ;[0 0 0] Create Skills Menu Widget and add it to the viewport(Don't remove the 0 second delay)
  (bind _returnvalue (UserInterface|CreateWidget "/Game/Dynamic_Skill_Tree_System/Widgets/WBP_SkillsMenu.WBP_SkillsMenu_C"))
  (bind _output_get (Variables|Default|SetWBP_SkillsMenu _returnvalue))
  (Utilities|FlowControl|Delay 0.0)
  (UserInterface|Viewport|AddtoViewport _output_get 0))

(event EventOpen/CloseSkillsMenu
  (params (Open :type Boolean))
  (bind _returnvalue (Game|GetPlayerController 0))
  (bind _returnvalue_2 (Game|GetPlayerController 0))
  (bind _wbp_skillsmenu (Variables|Default|GetWBP_SkillsMenu))
  ;[0 0 0] Open/Close the Skills Menu
  (Variables|Default|GetWBP_SkillsMenu
    (:then
      (if Open
        (if (Widget|IsVisible (Variables|Default|GetWBP_SkillsMenu))
          (Class|BISkillsFunction|Open/CloseSkillsMenu(Message) _wbp_skillsmenu true)
          (else
            (UserInterface|Viewport|AddtoViewport _wbp_skillsmenu 0)))
        (Variables|/Script/Engine.PlayerController|SetbShowMouseCursor _returnvalue_2 true)
        (Input|SetInputModeGameandUI _returnvalue_2 0 "DoNotLock" true false)
        (Game|SetGamePaused true)
        (else
          (Class|BISkillsFunction|Open/CloseSkillsMenu(Message) (Variables|Default|GetWBP_SkillsMenu) false)
          (Variables|/Script/Engine.PlayerController|SetbShowMouseCursor _returnvalue false)
          (Input|SetInputModeGameOnly _returnvalue false)
          (Game|SetGamePaused false))))
    (:else)))

(event EventSetSkillDetailsInfo
  (params (Skill :type F%20Skill%20Details%20Structure))
  ;[0 0 0] Set Skill Details Info
  (bind _skill_details (Class|BISkillsFunction|GetSkillDetailsWidget(Message) (Variables|Default|GetWBP_SkillsMenu)))
  (Class|BISkillsFunction|SetSkillDetailsInfo(Message) _skill_details Skill))

(fn ConstructionScript)

(fn GetSkillDetailsWidget
  (return 0))

(fn GetSkillMenu
  (return 0))

(fn IsSkillsMenuOpen
  (bind _open (Class|BISkillsFunction|IsSkillsMenuOpen(Message) (Variables|Default|GetWBP_SkillsMenu)))
  (return _open))