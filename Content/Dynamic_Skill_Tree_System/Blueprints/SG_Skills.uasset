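; SG_Skills is the SaveGame object that persists the skill tree, with functions to save, load and delete its own data.
; Saving a skill copies both maps from the "Skills" slot, updates SkillsMap, and rebuilds SkillsStageMap entries by AltName, re-adding only purchased skills.
; Skill points save separately to the "Skill Tree Component" slot.
; Deletion clears both slots plus a "Vitality" slot.
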(fn SaveSkillDetails
  (params (Skill%20Name :type Name) (Skill%20Details :type F%20Skill%20Details%20Structure))
  (bind _returnvalue (SaveGame|DoesSaveGameExist "Skills"))
  (if _returnvalue
    (bind _returnvalue_2 (SaveGame|LoadGamefromSlot "Skills"))
    (bind _assg_skills (Utilities|Casting|CastToSG_Skills _returnvalue_2))
    (Variables|Skills|Private|SetSkills%20Map (Variables|SG_Skills_C|GetSkills%20Map _assg_skills))
    (Variables|Skills|Private|SetSkills%20Stage%20Map (Variables|SG_Skills_C|GetSkills%20Stage%20Map _assg_skills)))
  (Utilities|FlowControl|Sequence
    (:then_0
      (if (Utilities|Map|Contains (Variables|Skills|Private|GetSkills%20Map) Skill%20Name)
        (Utilities|Map|Remove (Variables|Skills|Private|GetSkills%20Map) Skill%20Name)
        (Utilities|Map|Add (Variables|Skills|Private|GetSkills%20Map) Skill%20Name Skill%20Details)
        (SaveGame|SaveGametoSlot self "Skills")
        (else
          (Utilities|Map|Add (Variables|Skills|Private|GetSkills%20Map) Skill%20Name Skill%20Details)
          (SaveGame|SaveGametoSlot self "Skills"))))
    (:then_1
      (bind _keys (Utilities|Map|Keys (Variables|Skills|Private|GetSkills%20Stage%20Map)))
      (for _array_element _keys
        (if (Utilities|Enum|Equal(Enum) (Utilities|Struct|BreakF_SkillDetails (.Value (Utilities|Map|Find (Variables|Skills|Private|GetSkills%20Stage%20Map) _array_element))) (Utilities|Struct|BreakF_SkillDetails Skill%20Details))
          (Utilities|Map|Remove (Variables|Skills|Private|GetSkills%20Stage%20Map) _array_element)))
      (if (Utilities|Struct|BreakF_SkillDetails Skill%20Details)
        (Utilities|Map|Add (Variables|Skills|Private|GetSkills%20Stage%20Map) Skill%20Name Skill%20Details)
        (SaveGame|SaveGametoSlot self "Skills")))))

(fn LoadSkillDetails
  (params (Skill :type Name))
  (bind _returnvalue (SaveGame|DoesSaveGameExist "Skills"))
  (if _returnvalue
    (bind _returnvalue_2 (SaveGame|LoadGamefromSlot "Skills"))
    (bind _assg_skills (Utilities|Casting|CastToSG_Skills _returnvalue_2))
    (bind _output_get (LocalVariables|SetLV%20Save%20REF _assg_skills))
    (return (.ReturnValue (Utilities|Map|Find (Variables|SG_Skills_C|GetSkills%20Map _output_get) Skill)) (.Value (Utilities|Map|Find (Variables|SG_Skills_C|GetSkills%20Map _output_get) Skill)))
    (else
      (return false ""))))

(fn LoadSkillsComponent
  (bind _returnvalue (SaveGame|DoesSaveGameExist "Skill Tree Component"))
  (if _returnvalue
    (bind _returnvalue_2 (SaveGame|LoadGamefromSlot "Skill Tree Component"))
    (bind _assg_skills (Utilities|Casting|CastToSG_Skills _returnvalue_2)
      (:then
        (return true (Variables|SG_Skills_C|GetSkill%20Points _assg_skills)))
      (:CastFailed
        (return false 0)))
    (else
      (return false 0))))

(fn SaveSkillsComponent
  (params (Skill%20Points :type Integer))
  (Variables|SkillsComponent|Private|SetSkill%20Points Skill%20Points)
  (SaveGame|SaveGametoSlot self "Skill Tree Component"))

(fn LoadAllSkillDetails
  (bind _returnvalue (SaveGame|DoesSaveGameExist "Skills"))
  (if _returnvalue
    (bind _returnvalue_2 (SaveGame|LoadGamefromSlot "Skills"))
    (bind _assg_skills (Utilities|Casting|CastToSG_Skills _returnvalue_2)
      (:then
        (bind _output_get (LocalVariables|SetLV%20Save%20REF _assg_skills))
        (return true (Variables|SG_Skills_C|GetSkills%20Map _output_get) (Variables|SG_Skills_C|GetSkills%20Stage%20Map _output_get)))
      (:CastFailed
        (return false 0 0)))
    (else
      (return false 0 0))))

(fn DeleteSaveFiles
  (SaveGame|DeleteGameinSlot "Skills")
  (SaveGame|DeleteGameinSlot "Skill Tree Component")
  (SaveGame|DeleteGameinSlot "Vitality"))