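; Actor component for a skill tree that saves skill points and applies purchased skill upgrades to its owner.
; On BeginPlay it loads SG_Skills and replays each saved skill stage through OnSkillPurchased, which W_Skill also calls on purchase.
; Skill names map to staged health, armor, regeneration and speed setters on AC_VitalityComponent and CharacterMovement.
; It also toggles the skills menu via PlayerController messages and deletes saves on R; ResetSkills is an empty stub.
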(event Custom|Save%20Skills%20Component
  ;[0 0 0] Save variables inside component
  (Utilities|IsValid (Variables|Private|References|GetSave%20REF)
    (:Is%20Valid
      _)
    (:Is%20Not%20Valid
      (bind _returnvalue (SaveGame|CreateSaveGameObject "/Game/Dynamic_Skill_Tree_System/Blueprints/SG_Skills.SG_Skills_C"))
      (Variables|Private|References|SetSave%20REF _returnvalue)))
  (Default|SaveSkillsComponent (Variables|Private|References|GetSave%20REF) (Variables|Default|GetSkill%20Points)))

(event Custom|Load%20Skills%20Component
  ;[0 0 0] Load variables inside component and set them
  (Utilities|IsValid (Variables|Private|References|GetSave%20REF)
    (:Is%20Valid
      _)
    (:Is%20Not%20Valid
      (bind _returnvalue (SaveGame|CreateSaveGameObject "/Game/Dynamic_Skill_Tree_System/Blueprints/SG_Skills.SG_Skills_C"))
      (Variables|Private|References|SetSave%20REF _returnvalue)))
  (Utilities|FlowControl|Sequence
    (:then_0
      (bind (_returnvalue_2 _skills_map _skills_stage_map) (Default|LoadAllSkillDetails (Variables|Private|References|GetSave%20REF)))
      (if _returnvalue_2
        (Variables|Private|SetSkills%20Map _skills_map)
        (Variables|Private|SetSkills%20Stage%20Map _skills_stage_map)
        (CallFunction|ApplySkills)))
    (:then_1
      (bind (_load_successful _skill_points) (Default|LoadSkillsComponent (Variables|Private|References|GetSave%20REF)))
      (if _load_successful
        (Variables|Default|SetSkill%20Points _skill_points)))))

(event Custom|Delete%20Save%20Files
  ;[0.004833 1 0] Call this event to reset every thing back
  (Utilities|IsValid (Variables|Private|References|GetSave%20REF)
    (:Is%20Valid
      _)
    (:Is%20Not%20Valid
      (bind _returnvalue (SaveGame|CreateSaveGameObject "/Game/Dynamic_Skill_Tree_System/Blueprints/SG_Skills.SG_Skills_C"))
      (Variables|Private|References|SetSave%20REF _returnvalue)))
  (Default|DeleteSaveFiles (Variables|Private|References|GetSave%20REF)))

(event Input|EnhancedActionEvents|EnhancedInputActionIA_Open_SkillsMenu
  (params (ActionValue :type Boolean) (ElapsedSeconds :type Float%20%28double-precision%29) (TriggeredSeconds :type Float%20%28double-precision%29) (InputAction :type Input%20Action%20Object%20Reference :default "/Game/Dynamic_Skill_Tree_System/Demo/Demo_Character/Input/Actions/IA_Open_SkillsMenu.IA_Open_SkillsMenu"))
  (bind _returnvalue (Game|GetPlayerController 0))
  ;[0 0 0] Open/Close W_SkillsMenu
  (:Triggered
    (bind _open (Class|BISkillsFunction|IsSkillsMenuOpen(Message) (Game|GetPlayerController 0)))
    (if _open
      (Class|BISkillsFunction|Open/CloseSkillsMenu(Message) _returnvalue false)
      (else
        (Class|BISkillsFunction|Open/CloseSkillsMenu(Message) _returnvalue true)))))

(event EventBeginPlay
  ;[0 0 0] Load skills and create W_SkillsMenu and set a reference var
  (CallFunction|LoadSkillsComponent))

(event EventOnSkillPurchased
  (params (Alt%20Name :type String) (Stage :type Integer))
  ;[0 0 0] When the player purchases a skill, it will call this event. This is where you store the functionality for applying skills
  ;;[0.04688 0.04688 0.04688] Called from W_Skill Widget inside of the "Purchase Skill" Function
  (switch string Alt%20Name
    (:Health%20Multiplier
      (Private|SetHealthMultiplier Stage))
    (:Armor%20Multiplier
      (Private|SetArmorMultiplier Stage))
    (:Speed%20Multiplier
      (Private|SetSpeedMultiplier Stage))
    (:Health%20Regeneration
      (Private|SetHealthRegeneration Stage))))

(event Input|KeyboardEvents|R
  (params (Key :type Key%20Structure :default "None"))
  ;[0.01767 1 0] click play and hit "R" to delete Save Files (used to reset all of the skills). You can have this on beginplay to delete save files everytime you run the game
  (:Pressed
    (CallFunction|DeleteSaveFiles)))

(fn SetHealthMultiplier
  (params (Stage :type Integer))
  (switch int Stage
    (:Default
      (LocalVariables|SetLV%20Health%20Multiplier 1.0))
    (:1
      (LocalVariables|SetLV%20Health%20Multiplier 1.25))
    (:2
      (LocalVariables|SetLV%20Health%20Multiplier 1.5))
    (:3
      (LocalVariables|SetLV%20Health%20Multiplier 1.75))
    (:4
      (LocalVariables|SetLV%20Health%20Multiplier 2.0)))
  (Default|SetHealthMultiplier (Actor|GetComponentbyClass (Components|GetOwner) "/Game/Dynamic_Skill_Tree_System/Demo/VitalitySystem/Blueprints/AC_VitalityComponent.AC_VitalityComponent_C") (LocalVariables|GetLV%20Health%20Multiplier)))

(fn SetArmorMultiplier
  (params (Stage :type Integer))
  (switch int Stage
    (:Default
      (LocalVariables|SetLV%20Armor%20Multiplier 1.0))
    (:1
      (LocalVariables|SetLV%20Armor%20Multiplier 1.25))
    (:2
      (LocalVariables|SetLV%20Armor%20Multiplier 1.5))
    (:3
      (LocalVariables|SetLV%20Armor%20Multiplier 1.75))
    (:4
      (LocalVariables|SetLV%20Armor%20Multiplier 2.0)))
  (Default|SetArmorMultiplier (Actor|GetComponentbyClass (Components|GetOwner) "/Game/Dynamic_Skill_Tree_System/Demo/VitalitySystem/Blueprints/AC_VitalityComponent.AC_VitalityComponent_C") (LocalVariables|GetLV%20Armor%20Multiplier)))

(fn ApplySkills
  (bind _keys (Utilities|Map|Keys (Variables|Private|GetSkills%20Stage%20Map)))
  (for _array_element _keys
    ;[0 0 0] Used to apply skills that have been purchased
    (CallFunction|OnSkillPurchased (.AltName (Utilities|Struct|BreakF_SkillDetails (.Value (Utilities|Map|Find (Variables|Private|GetSkills%20Stage%20Map) _array_element)))) (.Stage (Utilities|Struct|BreakF_SkillDetails (.Value (Utilities|Map|Find (Variables|Private|GetSkills%20Stage%20Map) _array_element)))))))

(fn SetSpeedMultiplier
  (params (Stage :type Integer))
  (bind _returnvalue (Components|GetOwner))
  (bind _returnvalue_2 (Actor|GetComponentbyClass _returnvalue "/Script/Engine.CharacterMovementComponent"))
  (switch int Stage
    (:Default
      (LocalVariables|SetLV%20Speed%20Multiplier 1.0))
    (:1
      (LocalVariables|SetLV%20Speed%20Multiplier 1.2))
    (:2
      (LocalVariables|SetLV%20Speed%20Multiplier 1.6))
    (:3
      (LocalVariables|SetLV%20Speed%20Multiplier 2.0)))
  (Variables|/Script/Engine.CharacterMovementComponent|SetMaxWalkSpeed _returnvalue_2 (* 6e+02 (LocalVariables|GetLV%20Speed%20Multiplier)))
  (Variables|/Script/Engine.CharacterMovementComponent|SetMaxWalkSpeedCrouched _returnvalue_2 (* 3e+02 (LocalVariables|GetLV%20Speed%20Multiplier))))

(fn SetHealthRegeneration
  (params (Stage :type Integer))
  (switch int Stage
    (:Default
      (Variables|/Game/Dynamic_Skill_Tree_System/Demo/VitalitySystem/Blueprints/AC_VitalityComponent.AC_VitalityComponent_C|SetHealth%20Regeneration (Actor|GetComponentbyClass (Components|GetOwner) "/Game/Dynamic_Skill_Tree_System/Demo/VitalitySystem/Blueprints/AC_VitalityComponent.AC_VitalityComponent_C") false)
      (LocalVariables|SetLV%20Health%20Regen%20Multiplier 1.0))
    (:1
      (Variables|/Game/Dynamic_Skill_Tree_System/Demo/VitalitySystem/Blueprints/AC_VitalityComponent.AC_VitalityComponent_C|SetHealth%20Regeneration (Actor|GetComponentbyClass (Components|GetOwner) "/Game/Dynamic_Skill_Tree_System/Demo/VitalitySystem/Blueprints/AC_VitalityComponent.AC_VitalityComponent_C") true))
    (:2
      (LocalVariables|SetLV%20Health%20Regen%20Multiplier 1.5))
    (:3
      (LocalVariables|SetLV%20Health%20Regen%20Multiplier 2.0)))
  (Default|SetHealthRegenMultiplier (Actor|GetComponentbyClass (Components|GetOwner) "/Game/Dynamic_Skill_Tree_System/Demo/VitalitySystem/Blueprints/AC_VitalityComponent.AC_VitalityComponent_C") (LocalVariables|GetLV%20Health%20Regen%20Multiplier)))

(fn AddSkillPoints
  (params (Amount :type Integer))
  (Variables|Default|SetSkill%20Points (+ (Variables|Default|GetSkill%20Points) Amount))
  (CallFunction|SaveSkillsComponent))

(fn ResetSkills)